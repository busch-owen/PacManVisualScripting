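; Pac-Man game mode that tracks score and lives and handles resetting after a death.
; BeginPlay caches each ghost's starting location in an array parallel to the Ghosts array.
; Losing a life either restarts the player at the player start and moves ghosts back to those locations, or reloads the level when lives run out.
; Score increases are added to the total and printed to screen.
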(event `self.ReceiveBeginPlay`
  (for (_array_element _array_index) (`self.Ghosts`)
    (`KismetArrayLibrary.Array_Set` (`self.GhostPositions`) _array_index (`self.K2_GetActorLocation` _array_element))))

(event `Restart Level`
  (`self.RestartPlayerAtPlayerStart` null)
  (for (_array_element _array_index) (`self.Ghosts`)
    (`self.K2_SetActorLocation` _array_element (`|GetArrayItem` (`self.GhostPositions`) _array_index) false false)))

(event `IncreaseScore`
  (params (IncreaseAmount :type Integer))
  (bind _output_get (set `self.Score` (+ IncreaseAmount (`self.Score`))))
  (`KismetSystemLibrary.PrintString` (`KismetStringLibrary.Conv_IntToString` _output_get)))

(event `LoseLife`
  (bind _result (`/Engine/EditorBlueprintResources/StandardMacros.DecrementInt` (`self.Lives`))
    (:`  `
      (if (<= _result 0)
        (`GameplayStatics.OpenLevel` (`KismetStringLibrary.Conv_StringToName` (`KismetSystemLibrary.GetObjectName` (`self.GetLevel`))))
        (else
          (`self.Restart Level`))))))

(fn `UserConstructionScript`)