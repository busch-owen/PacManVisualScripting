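; BP_GhostController is a controller that makes its possessed pawn, presumably a ghost, chase the first player's pawn.
; From BeginPlay, an endless loop calls FollowPlayer and waits one second between calls.
; FollowPlayer checks that the controlled pawn is valid, then issues AIMoveTo toward a snapshot of the player's location rather than tracking the actor.
; Move success or failure is only printed as debug text.
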(event `FollowPlayer`
  (bind _returnvalue (`self.K2_GetPawn`))
  (`/Engine/EditorBlueprintResources/StandardMacros.IsValid` _returnvalue
    (:`Is Valid`
      (`|AIMoveTo` _returnvalue (`self.K2_GetActorLocation` (`self.K2_GetPawn` (`GameplayStatics.GetPlayerController` 0))) null
        (:`OnSuccess`
          (`KismetSystemLibrary.PrintString` "Success"))
        (:`OnFail`
          (`KismetSystemLibrary.PrintString` "Failure"))))))

(event `self.ReceiveBeginPlay`
  (`self.FollowPlayer` :!label _label)
  (`KismetSystemLibrary.Delay` 1.0)
  (goto _label))

(fn `UserConstructionScript`)