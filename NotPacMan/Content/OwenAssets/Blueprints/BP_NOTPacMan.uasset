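; Player-controlled Pac-Man-style pawn that moves with Enhanced Input and loses a life on contact with a ghost.
; IA_Move drives movement along the actor's forward and right vectors and turns only the static mesh toward the input direction.
; Capsule overlap with BP_Ghost calls LoseLife on PacManGamemode, then destroys the pawn and has the game mode restart its controller.
; Destruction also notifies the game mode through CallOnPlayerDied.
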(event `EnhancedInput|/Game/OwenAssets/Input/IA_Move`
  (params (ActionValue :type "Vector2D Structure") (ElapsedSeconds :type "Float (double-precision)") (TriggeredSeconds :type "Float (double-precision)") (InputAction :type "InputAction Object Reference" :default "/Game/OwenAssets/Input/IA_Move.IA_Move"))
  (:`Triggered`
    (`self.AddMovementInput` (`self.GetActorRightVector`) (* ActionValue_X (`self.MoveSpeed`)))
    (`self.AddMovementInput` (`self.GetActorForwardVector`) (* ActionValue_Y (`self.MoveSpeed`)))
    (`SceneComponent.K2_SetWorldRotation` (`self.StaticMesh`) (`KismetMathLibrary.MakeRotFromX` (`KismetMathLibrary.MakeVector` ActionValue_X (* ActionValue_Y -1.0))) false false)))

(event `self.ReceiveBeginPlay`
  (bind _aspac_man_gamemode (cast `/Game/OwenAssets/Blueprints/PacManGamemode` (`GameplayStatics.GetGameMode`)))
  (set `self.PacManGamemode` _aspac_man_gamemode))

(event `self.CapsuleComponent.OnComponentBeginOverlap`
  (params (OverlappedComponent :type "PrimitiveComponent Object Reference") (OtherActor :type "Actor Object Reference") (OtherComp :type "PrimitiveComponent Object Reference") (OtherBodyIndex :type Integer) (bFromSweep :type Boolean) (SweepResult :type "HitResult Structure (by ref)"))
  (cast `/Game/OwenAssets/Blueprints/BP_Ghost` OtherActor)
  (`/Game/OwenAssets/Blueprints/PacManGamemode.LoseLife` (`self.PacManGamemode`))
  (`self.CallRestartPlayer`))

(event `self.ReceiveDestroyed`
  (bind _aspac_man_gamemode (cast `/Game/OwenAssets/Blueprints/PacManGamemode` (`GameplayStatics.GetGameMode`)))
  (`/Game/OwenAssets/Blueprints/PacManGamemode.OnPlayerDied` _aspac_man_gamemode self))

(fn `CallRestartPlayer`
  (locals (ControllerRef :type "Controller Object Reference"))
  (set `local.ControllerRef` (`self.GetController`))
  (`self.K2_DestroyActor`)
  (bind _aspac_man_gamemode (cast `/Game/OwenAssets/Blueprints/PacManGamemode` (`GameplayStatics.GetGameMode`)))
  (`GameModeBase.RestartPlayer` _aspac_man_gamemode (`local.ControllerRef`)))

(fn `UserConstructionScript`)