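; Pac-Man game mode that tracks score and lives and handles ghost resets and level changes.
; BeginPlay caches every ghost's start position and creates a HUD widget inside that loop, so one per ghost.
; LoseLife returns ghosts to those positions or opens the main menu when lives run out, while a separate death event respawns the player.
; IncreaseScore loads level two once the score threshold is reached.
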(event `Restart Level`
  (for (_array_element _array_index) (`self.Ghosts`)
    (`self.K2_SetActorLocation` _array_element (`|GetArrayItem` (`self.GhostPositions`) _array_index) false false))
  (`KismetSystemLibrary.PrintString` "reset locations of all ghosts"))

(event `IncreaseScore`
  (params (IncreaseAmount :type Integer))
  (bind _output_get (set `self.Score` (+ IncreaseAmount (`self.Score`))))
  (`KismetSystemLibrary.PrintString` (`KismetStringLibrary.Conv_IntToString` _output_get))
  (if (>= (`self.Score`) 2090)
    (`GameplayStatics.OpenLevel` "Level_PacManLevel2")))

(event `LoseLife`
  (bind _result (`/Engine/EditorBlueprintResources/StandardMacros.DecrementInt` (`self.Lives`))
    (:`  `
      (if (< _result 0)
        (`GameplayStatics.OpenLevel` "Level_MainMenu")
        (else
          (`self.Restart Level`))))))

(event `self.ReceiveBeginPlay`
  (add `self.OnPlayerDied` (delegate `PlayerDied`))
  (bind _outactors (`GameplayStatics.GetAllActorsOfClass` "/Game/OwenAssets/Blueprints/BP_Ghost.BP_Ghost_C"))
  (bind _output_get (set `self.Ghosts` _outactors))
  (for (_array_element _array_index) _output_get
    (`KismetArrayLibrary.Array_Set` (`self.GhostPositions`) _array_index (`self.K2_GetActorLocation` _array_element) true)
    (bind _returnvalue (`|CreateWidget` "/Game/OwenAssets/Blueprints/BP_HUD.BP_HUD_C"))
    (bind _output_get_2 (set `self.PlayerHud` _returnvalue))
    (`UserWidget.AddToViewport` _output_get_2 0)))

(event `PlayerDied` :!signature `self.OnPlayerDied`
  (params (Character :type "Character Object Reference"))
  (`self.RestartPlayer` (`Pawn.GetController` Character)))

(fn `UserConstructionScript`)